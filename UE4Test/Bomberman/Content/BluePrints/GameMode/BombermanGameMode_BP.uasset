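; Game mode for a Bomberman game that runs the match countdown and triggers the game over screen.
; Tick uses a one-second Delay to step the Minutes and Seconds variables down.
; When time runs out or the GameOver flag is set, it adds GameOverScreen_UMG to the viewport, shows the mouse cursor and pauses the game.
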(event EventBeginPlay)

(event EventTick
  (params (DeltaSeconds :type Float%20%28single-precision%29))
  (if (Variables|Default|GetbGameOver)
    (bind _returnvalue (UserInterface|CreateWidget "/Game/BluePrints/Widgets/GameOverScreen_UMG.GameOverScreen_UMG_C" :!label _label))
    (UserInterface|Viewport|AddtoViewport _returnvalue 0)
    (Variables|/Script/Engine.PlayerController|SetbShowMouseCursor (Game|GetPlayerController 0) true)
    (Game|SetGamePaused true)
    (else
      (Utilities|FlowControl|Delay 1.0)
      (if (== (Variables|Default|GetSeconds) 0)
        (if (== (Variables|Default|GetMinutes) 0)
          (goto _label)
          (else
            (Variables|Default|SetSeconds 59)
            (Variables|Default|SetMinutes (- (Variables|Default|GetMinutes) 1))))
        (else
          (Variables|Default|SetSeconds (- (Variables|Default|GetSeconds) 1)))))))

(fn ConstructionScript)